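; Interactive door actor that a player opens and closes with the E key while standing inside its trigger box.
; Box overlap by a player-controlled Character enables or disables the actor's input and shows or hides the inside and outside text prompts.
; E toggles IsOpen and plays or reverses a Timeline that drives the door's relative yaw, with an IsDoing flag blocking presses mid-swing.
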(event OnComponentBeginOverlap(Box)
  (params (OverlappedComponent :type Primitive%20Component%20Object%20Reference) (OtherActor :type Actor%20Object%20Reference) (OtherComp :type Primitive%20Component%20Object%20Reference) (OtherBodyIndex :type Integer) (bFromSweep :type Boolean) (SweepResult :type Hit%20Result%20Structure%20%28by%20ref%29))
  (bind _ascharacter (Utilities|Casting|CastToCharacter OtherActor))
  (bind _asplayer_controller (Utilities|Casting|CastToPlayerController (Pawn|GetController _ascharacter)))
  (Input|EnableInput _asplayer_controller)
  (Rendering|SetVisibility (Variables|Default|GetTextRenderIn) true false))

(event OnComponentEndOverlap(Box)
  (params (OverlappedComponent :type Primitive%20Component%20Object%20Reference) (OtherActor :type Actor%20Object%20Reference) (OtherComp :type Primitive%20Component%20Object%20Reference) (OtherBodyIndex :type Integer))
  (bind _ascharacter (Utilities|Casting|CastToCharacter OtherActor))
  (bind _asplayer_controller (Utilities|Casting|CastToPlayerController (Pawn|GetController _ascharacter)))
  (Input|DisableInput _asplayer_controller)
  (Rendering|SetVisibility (Variables|Default|GetTextRenderIn) false false))

(event Input|KeyboardEvents|E
  (params (Key :type Key%20Structure))
  (:Pressed
    (if (not (Variables|Default|GetIsDoing))
      (if (Variables|Default|GetIsOpen)
        (Variables|Default|SetIsOpen false)
        (bind _newtrack_1 (Timeline|Timeline_0 Reverse)
          (:Update
            (Transformation|SetRelativeRotation (Variables|Default|GetDoor) (Math|Rotator|MakeRotator 0.0 0.0 _newtrack_1) false false)
            (Variables|Default|SetIsDoing true))
          (:Finished
            (Variables|Default|SetIsDoing false)))
        (else
          (Variables|Default|SetIsOpen true)
          (Timeline|Timeline_0 Play))))))

(fn ConstructionScript)