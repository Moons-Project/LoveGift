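; Interactable gift item that highlights when targeted, gets packaged and is then picked up.
; Reminder tip events swap the mesh material between selected and unselected.
; The first GetGift swaps the mesh to a cone; the next destroys the item and spawns a BoxGift at the player.
; DropGift destroys the carried gift when flags allow, but the attach-to-player and IsCarrying logic is disconnected.
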(event EventInteractReminderTips
  (Rendering|Material|SetMaterial (Variables|Default|GetStaticMesh) 0 "/Game/Metrials/M_IsSelected.M_IsSelected"))

(event EventInteractGetGift
  (if (Variables|Default|GetIsPackaged?)
    (Actor|DestroyActor)
    (bind _returnvalue (Game|SpawnActorfromClass "/Game/Levels/BluePrints/BoxGift.BoxGift_C" (Transformation|GetActorTransform (Game|GetPlayerCharacter 0)) "Undefined" 0 0))
    (bind _output_get (Variables|Default|SetCarryingGift _returnvalue))
    (else
      (Components|StaticMesh|SetStaticMesh (Variables|Default|GetStaticMesh) "/Engine/BasicShapes/Cone.Cone")
      (Variables|Default|SetIsPackaged? true))))

(event EventInteractDropGift
  (if (Variables|Default|GetIsCarrying?)
    (if (Variables|Default|GetIsAbleToDrop?)
      (Actor|DestroyActor (Variables|Default|GetCarryingGift)))))

(event EventInteractReminderTipsClose
  (Rendering|Material|SetMaterial (Variables|Default|GetStaticMesh) 0 "/Game/Metrials/M_NotSelected.M_NotSelected"))

(fn ConstructionScript)